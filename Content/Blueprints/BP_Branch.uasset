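; BP_Branch is a tapering branch built from spline mesh segments along a spline.
; The construction script adds a colliding segment every SectionLength, clamping tangents to that length, shrinking thickness exponentially by ThicknessFalloff and closing the last segment to a point.
; On BeginPlay it spawns actors at interior spline points from index 2 onward, passing on its mesh and settings with a root thickness reduced by point index.
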(event `self.ReceiveBeginPlay`
  (bind _spline (`self.Spline`))
  (bind _returnvalue (`SplineComponent.GetNumberOfSplinePoints` (`self.Spline`)))
  (if (> _returnvalue 2)
    (for _index (range 2 (+ (- _returnvalue 2) 1))
      (bind _returnvalue_x (`KismetMathLibrary.BreakVector2D` (`self.GetScaleForSectionIndex` (+ _index 6))))
      (`|SpawnActorFromClass` "BP_Branch_C" (`KismetMathLibrary.MakeTransform` (`SplineComponent.GetLocationAtSplinePoint` _spline _index "World") (`SplineComponent.GetRotationAtSplinePoint` _spline _index "World")) "Undefined" "OverrideRootScale" self (`self.Mesh`) (`self.SectionLength`) (* (`self.RootThickness`) _returnvalue_x) (`self.ThicknessFalloff`) null))))

(fn `CreateSplineComponent`
  (returns (SplineComponent :type "SplineMeshComponent Object Reference"))
  (bind _returnvalue (`AddComponent|NODE_AddSplineMeshComponent-0`))
  (`PrimitiveComponent.SetCollisionEnabled` _returnvalue "QueryAndPhysics")
  (`StaticMeshComponent.SetStaticMesh` _returnvalue (`self.Mesh`))
  (`SplineMeshComponent.SetForwardAxis` _returnvalue "Z" true)
  (return _returnvalue))

(fn `GetScaleForSectionIndex`
  (params (Index :type Integer))
  (returns (ReturnValue :type "Vector2D Structure"))
  (bind _returnvalue (* (`self.RootThickness`) (`KismetMathLibrary.MultiplyMultiply_FloatFloat` (`self.ThicknessFalloff`) (+ Index 1))))
  (return (`KismetMathLibrary.MakeVector2D` _returnvalue _returnvalue)))

(fn `GetSplineInfoByDistanceAtSectionIndex`
  (params (SectionIndex :type Integer))
  (returns (Location :type "Vector Structure") (Tangent :type "Vector Structure"))
  (bind _spline (`self.Spline`))
  (bind _returnvalue (* SectionIndex (`self.SectionLength`)))
  (return (`SplineComponent.GetLocationAtDistanceAlongSpline` _spline _returnvalue "Local") (`KismetMathLibrary.ClampVectorSize` (`SplineComponent.GetTangentAtDistanceAlongSpline` _spline _returnvalue "Local") 0.0 (`self.SectionLength`))))

(fn `UserConstructionScript`
  (bind _returnvalue (`KismetMathLibrary.FTrunc` (/ (`SplineComponent.GetSplineLength` (`self.Spline`)) (`self.SectionLength`))))
  (for _index (range (+ _returnvalue 1))
    (bind _splinecomponent (`self.CreateSplineComponent`))
    (bind (_location _tangent) (`self.GetSplineInfoByDistanceAtSectionIndex` _index))
    (bind (_location_2 _tangent_2) (`self.GetSplineInfoByDistanceAtSectionIndex` (+ _index 1)))
    (`SplineMeshComponent.SetStartAndEnd` _splinecomponent _location _tangent _location_2 _tangent_2 true)
    (`SplineMeshComponent.SetStartScale` _splinecomponent (`self.GetScaleForSectionIndex` _index) true)
    (`SplineMeshComponent.SetEndScale` _splinecomponent (select `bool` (== _index _returnvalue) :`false` (`self.GetScaleForSectionIndex` (+ _index 1)) :`true` (0.0 0.0)) true)))