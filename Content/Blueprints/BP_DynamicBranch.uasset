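; BP_DynamicBranch is a branch that animates its growth along a spline when play begins.
; The construction script flattens the start and end points to X=0, writes them into the spline and builds the spline mesh.
; A timeline slides the mesh's time window along the spline, tapering it from root thickness by a falloff factor.
; When the timeline finishes, it notifies the player controller that the branch has finished animating.
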(event `self.ReceiveBeginPlay`
  (`self.GrowEndToPosition`))

(event `GrowEndToPosition`
  (bind (_direction _alpha) (`Timeline|GrowTimeline` :!via `PlayFromStart`)
    (:`Update`
      (set `self.Offset` _alpha)
      (`self.UpdateMesh`))
    (:`Finished`
      (`/Game/Blueprints/Framework/BP_PlayerController.BranchFinishedAnimating` (`/Game/Blueprints/Framework/BPFL_Globals.GetQualifiedPlayerController` 0)))))

(event `UpdateMesh`
  (bind _returnvalue (`self.GetEndThickness`))
  (bind _spline (`self.Spline`))
  (bind _rootthickness (`self.RootThickness`))
  (bind _returnvalue_2 (+ (`self.Offset`) (`self.TimeStart`)))
  (bind _returnvalue_3 (+ (`self.Offset`) (`self.TimeEnd`)))
  (`SplineMeshComponent.SetStartAndEnd` (`self.SplineMesh`) (`SplineComponent.GetLocationAtTime` _spline _returnvalue_2 "Local" true) (`SplineComponent.GetTangentAtTime` _spline _returnvalue_2 "Local" true) (`SplineComponent.GetLocationAtTime` _spline _returnvalue_3 "Local" true) (`SplineComponent.GetTangentAtTime` _spline _returnvalue_3 "Local" true) true)
  (`SplineMeshComponent.SetStartScale` (`self.SplineMesh`) (`KismetMathLibrary.MakeVector2D` _rootthickness _rootthickness) true)
  (`SplineMeshComponent.SetEndScale` (`self.SplineMesh`) (`KismetMathLibrary.MakeVector2D` _returnvalue _returnvalue) true))

(fn `GetEndThickness`
  (returns (ReturnValue :type "Float (double-precision)"))
  (return (* (`self.RootThickness`) (`self.ThicknessFalloff`))))

(fn `UserConstructionScript`
  (bind _spline (`self.Spline`))
  (set `self.StartPoint` (`KismetMathLibrary.MakeVector` 0.0 (.y (`self.StartPoint`)) (.z (`self.StartPoint`))))
  (set `self.EndPoint` (`KismetMathLibrary.MakeVector` 0.0 (.y (`self.EndPoint`)) (.z (`self.EndPoint`))))
  (`SplineComponent.SetLocationAtSplinePoint` (`self.Spline`) 0 (`self.EndPoint`) "World" true)
  (`SplineComponent.SetLocationAtSplinePoint` _spline (`SplineComponent.GetNumberOfSplinePoints` _spline) (`self.StartPoint`) "World" true)
  (`self.UpdateMesh`))