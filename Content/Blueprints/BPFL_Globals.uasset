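; Blueprint function library that gives access to the game's global config and events through the game mode.
; GetQualifiedGameMode casts the current game mode to BP_GameMode, returning it only when the cast succeeds.
; GetGlobalConfig and GetGlobalEvents build on that helper to return the GlobalConfig and GlobalEvents members held by BP_GameMode.
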(fn `GetGlobalConfig`
  (returns (GlobalConfig :type "/Game/Blueprints/BP_GlobalConfig Object Reference"))
  (return (`/Game/Blueprints/BP_GameMode.GlobalConfig` (`self.GetQualifiedGameMode` (`local.__WorldContext`)))))

(fn `GetGlobalEvents`
  (returns (GlobalEvents :type "/Game/Blueprints/BP_GlobalEvents Object Reference"))
  (return (`/Game/Blueprints/BP_GameMode.GlobalEvents` (`self.GetQualifiedGameMode` (`local.__WorldContext`)))))

(fn `GetQualifiedGameMode`
  (returns (GameMode :type "/Game/Blueprints/BP_GameMode Object Reference"))
  (bind _asbp_game_mode (cast `/Game/Blueprints/BP_GameMode` (`GameplayStatics.GetGameMode` (`local.__WorldContext`))))
  (return _asbp_game_mode))