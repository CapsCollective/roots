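; BPFL_Globals is a Blueprint function library that gives typed access to core framework objects.
; It returns the game mode cast to BP_GameMode and the player controller at a given index cast to BP_PlayerController.
; GetGlobalConfig builds on the game mode getter to return the GlobalConfig stored on BP_GameMode.
; Both casts stop without returning a result when the active class does not match.
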(fn `GetGlobalConfig`
  (returns (GlobalConfig :type "/Game/Blueprints/Framework/BP_GlobalConfig Object Reference"))
  (return (`/Game/Blueprints/Framework/BP_GameMode.GlobalConfig` (`self.GetQualifiedGameMode` (`local.__WorldContext`)))))

(fn `GetQualifiedGameMode`
  (returns (GameMode :type "/Game/Blueprints/Framework/BP_GameMode Object Reference"))
  (bind _asbp_game_mode (cast `/Game/Blueprints/Framework/BP_GameMode` (`GameplayStatics.GetGameMode` (`local.__WorldContext`))))
  (return _asbp_game_mode))

(fn `GetQualifiedPlayerController`
  (params (PlayerIndex :type Integer))
  (returns (PlayerController :type "/Game/Blueprints/Framework/BP_PlayerController Object Reference"))
  (bind _asbp_player_controller (cast `/Game/Blueprints/Framework/BP_PlayerController` (`GameplayStatics.GetPlayerController` (`local.__WorldContext`) PlayerIndex)))
  (return _asbp_player_controller))