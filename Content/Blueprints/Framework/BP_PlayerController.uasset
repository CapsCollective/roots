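; Player controller that runs the grow-point expansion game: it shows the main overlay, enables cursor input and handles grow-point clicks.
; A click on an affordable, inactive point applies its cost and resource yield before the adjacency check.
; Activation requires an activated neighbour, except for the first point, which activates from itself.
; After each activation it prints a win on the final point, or a loss when no affordable, connected point remains.
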(event `self.ReceiveBeginPlay`
  (bind _returnvalue (`|CreateWidget` "/Game/Blueprints/UI/WBP_MainOverlay.WBP_MainOverlay_C"))
  (`UserWidget.AddToViewport` _returnvalue 0)
  (`WidgetBlueprintLibrary.SetInputMode_GameAndUIEx` self _returnvalue "DoNotLock" false)
  (set `self.bShowMouseCursor` true)
  (add `self.GrowPointClicked` (delegate `OnGrowPointClicked`)))

(event `OnGrowPointClicked` :!signature `self.GrowPointClicked`
  (params (GrowPoint :type "/Game/Blueprints/BP_GrowPoint Object Reference"))
  (bind (_isaffordable _updatedresources) (`self.IsAffordable` GrowPoint))
  (bind (_returnvalue _neighbour) (`self.HasRequiredNeighbour` GrowPoint))
  (if (`/Game/Blueprints/BP_GrowPoint.HasBeenActivated` GrowPoint)
    _
    (elif _isaffordable
      (set `self.CurrentResources` (`/Game/Blueprints/BPFL_Gameplay.AddResourceSets` _updatedresources (`/Game/Blueprints/BP_GrowPoint.Resources` GrowPoint)))
      (if _returnvalue
        (`/Game/Blueprints/BP_GrowPoint.Activate` GrowPoint _neighbour)
        (`KismetArrayLibrary.Array_AddUnique` (`self.ActivatedGrowPoints`) GrowPoint :!label _label)
        (if (`/Game/Blueprints/BP_GrowPoint.IsFinalGrowPoint` GrowPoint)
          (`KismetSystemLibrary.PrintString` "PLAYER WINS" true true (struct :`R` 0.061115 :`G` 1.0 :`A` 1.0))
          (elif (`self.IsPlayerLocked`)
            (`KismetSystemLibrary.PrintString` "LOST GAME - PLAYER LOCKED" true true (struct :`R` 1.0 :`G` 0.016184 :`A` 1.0))))
        (elif (`KismetArrayLibrary.Array_IsEmpty` (`self.ActivatedGrowPoints`))
          (`/Game/Blueprints/BP_GrowPoint.Activate` GrowPoint GrowPoint)
          (goto _label)))
      (else
        (`KismetSystemLibrary.PrintString` "Insufficient resources" true true (struct :`R` 1.0 :`G` 0.680463 :`B` 0.031698 :`A` 1.0))))))

(fn `HasRequiredNeighbour`
  (params (Target :type "/Game/Blueprints/BP_GrowPoint Object Reference"))
  (returns (ReturnValue :type Boolean) (Neighbour :type "/Game/Blueprints/BP_GrowPoint Object Reference"))
  (for _array_element (`self.ActivatedGrowPoints`)
    (if (`KismetArrayLibrary.Array_Contains` (`/Game/Blueprints/BP_GrowPoint.Neighbours` Target) _array_element)
      (return true _array_element))))

(fn `IsAffordable`
  (params (GrowPoint :type "/Game/Blueprints/BP_GrowPoint Object Reference"))
  (returns (IsAffordable :type Boolean) (UpdatedResources :type "/Game/Blueprints/S_ResourceSet Structure"))
  (bind _return_value (`/Game/Blueprints/BPFL_Gameplay.SubtractResourceSets` (`self.CurrentResources`) (`/Game/Blueprints/BP_GrowPoint.Cost` GrowPoint)))
  (return (`/Game/Blueprints/BPFL_Gameplay.IsResourceSetValid` _return_value) _return_value))

(fn `IsPlayerLocked`
  (returns (ReturnValue :type Boolean))
  (bind _outactors (`GameplayStatics.GetAllActorsOfClass` "/Game/Blueprints/BP_GrowPoint.BP_GrowPoint_C"))
  (for _array_element _outactors
    (bind _asbp_grow_point (cast `/Game/Blueprints/BP_GrowPoint` _array_element))
    (if (and (not (`/Game/Blueprints/BP_GrowPoint.HasBeenActivated` _asbp_grow_point)) (`self.IsAffordable` _asbp_grow_point) (`self.HasRequiredNeighbour` _asbp_grow_point))
      (return false)))
  (return true))

(fn `UserConstructionScript`
  (set `self.CurrentResources` (`/Game/Blueprints/Framework/BP_GlobalConfig.InitialPlayerResources` (`/Game/Blueprints/Framework/BPFL_Globals.GetGlobalConfig`))))