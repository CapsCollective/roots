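; Dialogue manager actor that plays timed dialogue sequences from a data table, currently the intro triggered by a grow point.
; On BeginPlay it listens to the player controller's grow point activation, and a point with the PlayIntro id starts the Intro row of DT_DialogueEvents.
; Playback sends the first line to the player controller, waits its display time, removes it and repeats, then signals dialogue ended.
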(event `self.ReceiveBeginPlay`
  (add `/Game/Blueprints/Framework/BP_PlayerController.GrowPointActivated` (`/Game/Blueprints/Framework/BPFL_Globals.GetQualifiedPlayerController` 0) (delegate `OnGrowPointActivated`)))

(event `OnGrowPointActivated`
  (params (GrowPoint :type "/Game/Blueprints/BP_GrowPoint Object Reference") (FromGrowPoint :type "/Game/Blueprints/BP_GrowPoint Object Reference"))
  (if (`/Game/Blueprints/BP_GrowPoint.HasId` GrowPoint "PlayIntro")
    (bind _returnvalue (`|GetDataTableRow` "/Game/Data/DT_DialogueEvents.DT_DialogueEvents" "Intro")
      (:`then`
        (`self.StartDialogueEvent` _returnvalue)))))

(event `StartDialogueEvent`
  (params (CurrentDialogueEvent :type "/Game/Blueprints/Structs/S_DialogueEvent Structure"))
  (bind _playercontroller (`/Game/Blueprints/Framework/BPFL_Globals.GetQualifiedPlayerController` 0))
  (bind _output_get (set `self.CurrentDialogueEvent` CurrentDialogueEvent))
  (bind _dialoguelines (break `/Game/Blueprints/Structs/S_DialogueEvent` _output_get))
  (if (`KismetArrayLibrary.Array_IsEmpty` _dialoguelines) :!label _label
    (set `self.CurrentDialogueEvent` (struct))
    (`/Game/Blueprints/Framework/BP_PlayerController.DialogueEnded` _playercontroller)
    (else
      (bind _output (`|GetArrayItem` _dialoguelines))
      (`/Game/Blueprints/Framework/BP_PlayerController.DialoguePlayed` _playercontroller _output)
      (`KismetSystemLibrary.Delay` (`.DisplayTime_5_553501095A47B58E401833B4F8319910` (break `/Game/Blueprints/Structs/S_DialogueLine` _output)))
      (`KismetArrayLibrary.Array_Remove` (`.DialogueLines_4_A2DA75BDCB4E5510285B4AA5054B639B` (break `/Game/Blueprints/Structs/S_DialogueEvent` (`self.CurrentDialogueEvent`))))
      (goto _label))))

(fn `UserConstructionScript`)