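; Gameplay function library with pure math helpers for orientation and for the game's Water and Iron resource sets.
; GetLookAtZ builds a rotation whose Z axis follows the normalized From minus To vector, so it points away from To.
; Resource sets are added and subtracted per field without clamping, and a separate validity check passes only when both amounts are non-negative.
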(fn `AddResourceSets`
  (params (ResourceSetA :type "/Game/Blueprints/S_ResourceSet Structure") (ResourceSetB :type "/Game/Blueprints/S_ResourceSet Structure"))
  (returns (`Return Value` :type "/Game/Blueprints/S_ResourceSet Structure"))
  (bind (_water _iron) (break `/Game/Blueprints/S_ResourceSet` ResourceSetB))
  (bind (_water_2 _iron_2) (break `/Game/Blueprints/S_ResourceSet` ResourceSetA))
  (return (make `/Game/Blueprints/S_ResourceSet` (+ _water_2 _water) (+ _iron_2 _iron))))

(fn `GetLookAtZ`
  (params (From :type "Vector Structure") (To :type "Vector Structure"))
  (returns (ReturnValue :type "Rotator Structure"))
  (return (`KismetMathLibrary.MakeRotFromZ` (`KismetMathLibrary.Normal` (- From To)))))

(fn `IsResourceSetValid`
  (params (ResourceSet :type "/Game/Blueprints/S_ResourceSet Structure"))
  (returns (`Return Value` :type Boolean))
  (bind (_water _iron) (break `/Game/Blueprints/S_ResourceSet` ResourceSet))
  (return (and (>= _water 0) (>= _iron 0))))

(fn `SubtractResourceSets`
  (params (ResourceSetA :type "/Game/Blueprints/S_ResourceSet Structure") (ResourceSetB :type "/Game/Blueprints/S_ResourceSet Structure"))
  (returns (`Return Value` :type "/Game/Blueprints/S_ResourceSet Structure"))
  (bind (_water _iron) (break `/Game/Blueprints/S_ResourceSet` ResourceSetB))
  (bind (_water_2 _iron_2) (break `/Game/Blueprints/S_ResourceSet` ResourceSetA))
  (return (make `/Game/Blueprints/S_ResourceSet` (- _water_2 _water) (- _iron_2 _iron))))