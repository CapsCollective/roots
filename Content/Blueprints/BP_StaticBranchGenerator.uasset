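; BP_StaticBranchGenerator spawns an actor, presumably a branch given the asset name, each time a grow point is clicked.
; On BeginPlay it binds to the grow-point-clicked event of the qualified player controller.
; Each spawn sits at the cached grow point with Z aimed at the clicked one, which then becomes cached, forming a chain.
; The first click caches itself before spawning, so its direction is zero.
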(event `self.ReceiveBeginPlay`
  (add `/Game/Blueprints/Framework/BP_PlayerController.GrowPointClicked` (`/Game/Blueprints/Framework/BPFL_Globals.GetQualifiedPlayerController` 0) (delegate `OnGrowPointClicked`)))

(event `OnGrowPointClicked`
  (params (GrowPoint :type "/Game/Blueprints/BP_GrowPoint Object Reference"))
  (`/Engine/EditorBlueprintResources/StandardMacros.IsValid` (`self.CachedGrowPoint`)
    (:`Is Valid`
      _)
    (:`Is Not Valid`
      (set `self.CachedGrowPoint` GrowPoint)))
  (`|SpawnActorFromClass` "/Game/Blueprints/Environment/BP_Plant.BP_Plant_C" (`KismetMathLibrary.MakeTransform` (`self.K2_GetActorLocation` (`self.CachedGrowPoint`)) (`KismetMathLibrary.MakeRotFromZ` (`KismetMathLibrary.Normal` (- (`self.K2_GetActorLocation` GrowPoint) (`self.K2_GetActorLocation` (`self.CachedGrowPoint`)))))) "Undefined" "OverrideRootScale" null null)
  (set `self.CachedGrowPoint` GrowPoint))

(fn `UserConstructionScript`)