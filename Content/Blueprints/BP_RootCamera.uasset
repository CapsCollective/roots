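; Camera actor that becomes the player's view target on BeginPlay and glides to grow points as they are clicked.
; It binds to the player controller's grow-point-clicked event, and each click stops any running move, caches the current position and restarts a Timeline.
; The Timeline lerps the actor toward the point's location in Y and Z only, keeping X fixed so the camera's depth stays constant.
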(event `self.ReceiveBeginPlay`
  (bind _playercontroller (`/Game/Blueprints/Framework/BPFL_Globals.GetQualifiedPlayerController` 0))
  (`PlayerController.SetViewTargetWithBlend` _playercontroller self 0.0 "VTBlend_Linear" 0.0 false)
  (add `/Game/Blueprints/Framework/BP_PlayerController.GrowPointClicked` _playercontroller (delegate `OnGrowPointClicked`)))

(event `OnGrowPointClicked`
  (params (GrowPoint :type "/Game/Blueprints/BP_GrowPoint Object Reference"))
  (`|ExecutionSequence`
    (:`then_0`
      (bind (_direction _alpha) (`Timeline|Timeline` :!via `Stop` :!label _label)
        (:`Update`
          (`self.K2_SetActorLocation` (`self.GetLerpedPosition` _alpha (`self.CachedPosition`) (stale `MoveToLocation` Location))))))
    (:`then_1`
      (`self.MoveToLocation` (`self.K2_GetActorLocation` GrowPoint)))))

(event `MoveToLocation`
  (params (Location :type "Vector Structure"))
  (set `self.CachedPosition` (`self.K2_GetActorLocation`))
  (goto _label :!via `PlayFromStart`))

(fn `GetLerpedPosition`
  (params (Alpha :type "Float (single-precision)") (A :type "Vector Structure") (B :type "Vector Structure"))
  (returns (ReturnValue :type "Vector Structure"))
  (return (`KismetMathLibrary.MakeVector` (.x A) (.y (`KismetMathLibrary.VLerp` A B Alpha)) (.z (`KismetMathLibrary.VLerp` A B Alpha)))))

(fn `UserConstructionScript`)