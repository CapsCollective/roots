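; BP_GrowPoint is a node in a graph of grow points that can be activated from one another.
; On BeginPlay it stores every grow point within the global config's neighbour radius, itself included, in Neighbours.
; It then briefly draws debug circles for the radius and node, plus arrows to each neighbour.
; Activate flags the point as activated and reports it and its source point to the player controller.
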(event `self.ReceiveBeginPlay`
  (bind _returnvalue (`self.K2_GetActorLocation`))
  (`|ExecutionSequence`
    (:`then_0`
      (bind _outactors (`GameplayStatics.GetAllActorsOfClass` "BP_GrowPoint_C"))
      (for _array_element _outactors
        (if (<= (`self.GetDistanceTo` _array_element self) (`/Game/Blueprints/Framework/BP_GlobalConfig.NodeMinimumNeighbourRadius` (`/Game/Blueprints/Framework/BPFL_Globals.GetGlobalConfig`)))
          (`KismetArrayLibrary.Array_Add` (`self.Neighbours`) _array_element))))
    (:`then_1`
      (`KismetSystemLibrary.DrawDebugCircle` _returnvalue (`/Game/Blueprints/Framework/BP_GlobalConfig.NodeMinimumNeighbourRadius` (`/Game/Blueprints/Framework/BPFL_Globals.GetGlobalConfig`)) 52 (struct :`R` 0.995748 :`B` 1.0 :`A` 1.0) 10.0 10.0)
      (`KismetSystemLibrary.DrawDebugCircle` _returnvalue 50.0 32 (struct :`G` 0.071725 :`B` 1.0 :`A` 1.0) 10.0 20.0)
      (for _array_element_2 (`self.Neighbours`)
        (`KismetSystemLibrary.DrawDebugArrow` _returnvalue (`self.K2_GetActorLocation` _array_element_2) 30.0 (struct :`R` 1.0 :`G` 0.019486 :`A` 1.0) 10.0 5.0)))))

(event `Activate`
  (params (FromGrowPoint :type "/Game/Blueprints/BP_GrowPoint Object Reference"))
  (set `self.HasBeenActivated` true)
  (`/Game/Blueprints/Framework/BP_PlayerController.GrowPointActivated` (`/Game/Blueprints/Framework/BPFL_Globals.GetQualifiedPlayerController` 0) self FromGrowPoint))

(fn `UserConstructionScript`)